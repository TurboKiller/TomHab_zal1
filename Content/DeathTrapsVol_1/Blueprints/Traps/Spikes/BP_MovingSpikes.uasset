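; BP_MovingSpikes is a spike trap that triggers the third-person character's death when that character overlaps its Box.
; BeginPlay, Tick and the construction script call the parent class, and this graph holds no movement logic of its own.
; The construction script then places the child actor at the start or end location according to the DirectionAnimation setting, with only Backward starting at the end.
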(event OnComponentBeginOverlap(Box)
  (params (OverlappedComponent :type Primitive%20Component%20Object%20Reference) (OtherActor :type Actor%20Object%20Reference) (OtherComp :type Primitive%20Component%20Object%20Reference) (OtherBodyIndex :type Integer) (bFromSweep :type Boolean) (SweepResult :type Hit%20Result%20Structure%20%28by%20ref%29))
  (bind _asbp_third_person_character (Utilities|Casting|CastToBP_ThirdPersonCharacter OtherActor))
  (Default|MainCharactterDatch _asbp_third_person_character))

(event EventBeginPlay
  (|CallParentFunction))

(event EventTick
  (params (DeltaSeconds :type Float%20%28single-precision%29))
  (|CallParentFunction DeltaSeconds))

(fn ConstructionScript
  (bind _locationstart (Variables|Default|GetLocationStart))
  (|CallParentFunction)
  ;[1 1 1] Set location by direction animation
  (Transformation|SetRelativeLocation (Variables|Default|GetBP_ChildActor) (Utilities|Select :Index (Variables|Default|GetDirectionAnimation) :NewEnumerator0 _locationstart :NewEnumerator1 _locationstart :NewEnumerator2 (Variables|Default|GetLocationEnd)) false false))