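; BP_MovingSpike is a moving spike trap that carries its spike as a child actor and inherits its runtime behavior from a parent class.
; The construction script sets the child actor's starting relative location from the animation direction: the end point for Backward, the start point for Forward and ForwardBackward.
; BeginPlay only calls the parent, and the file adds no movement logic of its own.
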(event EventBeginPlay
  (|CallParentFunction))

(event Collision|EventActorBeginOverlap
  (params (OtherActor :type Actor%20Object%20Reference)))

(event EventTick
  (params (DeltaSeconds :type Float%20%28single-precision%29))
  (|CallParentFunction DeltaSeconds) ; This node is disabled and will not be called.\nDrag off pins to build functionality.
)

(fn ConstructionScript
  (bind _locationstart (Variables|Default|GetLocationStart))
  (|CallParentFunction)
  ;[1 1 1] Set start location by direction animation
  (Transformation|SetRelativeLocation (Variables|Default|GetBP_ChildActor) (Utilities|Select :Index (Variables|Default|GetDirectionAnimation) :NewEnumerator0 _locationstart :NewEnumerator1 _locationstart :NewEnumerator2 (Variables|Default|GetLocationEnd)) false false))