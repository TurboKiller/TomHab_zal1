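; BP_OpenFloor is an open-floor trap from the DeathTraps pack that swings two meshes between start and end rotations.
; It builds on a parent Blueprint, forwarding Tick only while ActiveTrap is set.
; The AnimationLogic event lerps both meshes' relative rotations using FrameAnimation.X as alpha.
; The construction script snaps both meshes to their start or end rotation according to ForwardAnimation.
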(event EventBeginPlay
  (|CallParentFunction))

(event EventTick
  (params (DeltaSeconds :type Float%20%28single-precision%29))
  (if (Variables|Default|GetbActiveTrap)
    (|CallParentFunction DeltaSeconds)))

(event EventAnimationLogic
  ;[1 1 1] Rotate meshes
  (Transformation|SetRelativeRotation (Variables|Default|GetSM_Mesh_1) (Math|Rotator|Lerp(Rotator) (Variables|RotationByCurve|GetRotationStart_Mesh_1) (Variables|RotationByCurve|GetRotationEnd_Mesh_1) (.x (Variables|Default|GetFrameAnimation))) false false)
  (Transformation|SetRelativeRotation (Variables|Default|GetSM_Mesh_2) (Math|Rotator|Lerp(Rotator) (Variables|RotationByCurve|GetRotationStart_Mesh_2) (Variables|RotationByCurve|GetRotationEnd_Mesh_2) (.x (Variables|Default|GetFrameAnimation))) false false))

(fn ConstructionScript
  (|CallParentFunction)
  (Transformation|SetRelativeRotation (Variables|Default|GetSM_Mesh_1) (select (Variables|Default|GetbForwardAnimation) (Variables|RotationByCurve|GetRotationStart_Mesh_1) (Variables|RotationByCurve|GetRotationEnd_Mesh_1)) false false)
  (Transformation|SetRelativeRotation (Variables|Default|GetSM_Mesh_2) (select (Variables|Default|GetbForwardAnimation) (Variables|RotationByCurve|GetRotationStart_Mesh_2) (Variables|RotationByCurve|GetRotationEnd_Mesh_2)) false false))