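; Base trap Blueprint that slides a child-actor weapon module, such as spikes, between a start and end location.
; The construction script sets the weapon class and its initial position from the animation direction.
; BeginPlay passes damage and impulse settings to the weapon and swaps the endpoints for backward animation.
; AnimationLogic lerps the weapon's relative location using the X component of FrameAnimation.
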(event EventBeginPlay
  (|CallParentFunction)
  (Utilities|FlowControl|Sequence
    (:then_0
      ;[1 1 1] Set new damage settings
      (Utilities|IsValid (Variables|Default|GetBP_ChildActor)
        (:Is%20Valid
          (bind _asbp_base_module_weapon (Utilities|Casting|CastToBP_BaseModuleWeapon (Variables|/Script/Engine.ChildActorComponent|GetChildActor (Variables|Default|GetBP_ChildActor))))
          (Default|SetNewDamage _asbp_base_module_weapon (Variables|Default|GetDamage) (Variables|Default|GetImpulse) (Variables|Default|GetbCustomImpulse) (Variables|Default|GetDamageType)))))
    (:then_1
      ;[1 1 1] Swap variables
      (switch Utilities|FlowControl|Switch|SwitchonE_DirectionsAnimation (Variables|Default|GetDirectionAnimation)
        (:NewEnumerator2
          (Variables|Settings|Animation|LocationByCurve|SetTempLocationStart (Variables|Settings|Animation|LocationByCurve|GetLocationStart))
          (Variables|Settings|Animation|LocationByCurve|SetLocationStart (Variables|Settings|Animation|LocationByCurve|GetLocationEnd))
          (Variables|Settings|Animation|LocationByCurve|SetLocationEnd (Variables|Settings|Animation|LocationByCurve|GetTempLocationStart)))))))

(event EventTick
  (params (DeltaSeconds :type Float%20%28single-precision%29))
  (|CallParentFunction DeltaSeconds))

(event EventAnimationLogic
  ;[1 1 1] Change location spikes
  (Transformation|SetRelativeLocation (Variables|Default|GetBP_ChildActor) (Math|Vector|Lerp(Vector) (Variables|Settings|Animation|LocationByCurve|GetLocationStart) (Variables|Settings|Animation|LocationByCurve|GetLocationEnd) (.x (Variables|Default|GetFrameAnimation))) false false))

(fn ConstructionScript
  (|CallParentFunction)
  (ChildActorComponent|SetChildActorClass (Variables|Default|GetBP_ChildActor) (Variables|Settings|GetWeaponClass))
  (Transformation|SetRelativeLocation (Variables|Default|GetBP_ChildActor) (select (Variables|Default|GetbForwardAnimation) (Variables|Settings|Animation|LocationByCurve|GetLocationStart) (Variables|Settings|Animation|LocationByCurve|GetLocationEnd)) false false))