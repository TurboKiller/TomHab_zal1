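; Base rotation trap that swings a weapon module between two rotations.
; Construction spawns the chosen weapon class as a child actor and sets its initial rotation to one of the endpoints.
; BeginPlay passes damage, impulse and damage type to the weapon, and swaps the endpoints when the animation direction is Backward.
; AnimationLogic lerps the child actor's relative rotation using the X component of FrameAnimation.
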(event EventBeginPlay
  (|CallParentFunction)
  (Utilities|FlowControl|Sequence
    (:then_0
      ;[1 1 1] Set damage to weapon trap
      (bind _asbp_base_module_weapon (Utilities|Casting|CastToBP_BaseModuleWeapon (Variables|/Script/Engine.ChildActorComponent|GetChildActor (Variables|Default|GetBP_ChildActor))))
      (Default|SetNewDamage _asbp_base_module_weapon (Variables|Default|GetDamage) (Variables|Default|GetImpulse) (Variables|Default|GetbCustomImpulse) (Variables|Default|GetDamageType)))
    (:then_1
      ;[1 1 1] Swap variables
      (switch Utilities|FlowControl|Switch|SwitchonE_DirectionsAnimation (Variables|Default|GetDirectionAnimation)
        (:NewEnumerator2
          (Variables|Settings|Animation|RotationByCurve|SetTempRotationStart (Variables|Settings|Animation|RotationByCurve|GetRotationStart))
          (Variables|Settings|Animation|RotationByCurve|SetRotationStart (Variables|Settings|Animation|RotationByCurve|GetRotationEnd))
          (Variables|Settings|Animation|RotationByCurve|SetRotationEnd (Variables|Settings|Animation|RotationByCurve|GetTempRotationStart)))))))

(event EventAnimationLogic
  ;[1 1 1] Rotate mesh
  (Transformation|SetRelativeRotation (Variables|Default|GetBP_ChildActor) (Math|Rotator|Lerp(Rotator) (Variables|Settings|Animation|RotationByCurve|GetRotationStart) (Variables|Settings|Animation|RotationByCurve|GetRotationEnd) (.x (Variables|Default|GetFrameAnimation))) false false))

(event EventTick
  (params (DeltaSeconds :type Float%20%28single-precision%29))
  (|CallParentFunction DeltaSeconds))

(fn ConstructionScript
  (|CallParentFunction)
  (ChildActorComponent|SetChildActorClass (Variables|Default|GetBP_ChildActor) (Variables|Settings|GetWeaponClass)) ; Set weapon class
  ;[1 1 1] Start rotate weapon trap
  (Transformation|SetRelativeRotation (Variables|Default|GetBP_ChildActor) (select (Variables|Default|GetbForwardAnimation) (Variables|Settings|Animation|RotationByCurve|GetRotationEnd) (Variables|Settings|Animation|RotationByCurve|GetRotationStart)) false false))