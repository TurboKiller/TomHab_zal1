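; BP_RotationBlades is a blade trap that wraps a BP_Blades child actor and configures it from its own properties.
; Its Construction Script runs the parent script, then passes the blade count to the child and has it create the blades.
; It then applies the damage, impulse, custom impulse and damage type settings to those blades.
; The event graph only calls the parent BeginPlay, so it adds no runtime logic of its own.
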(event EventBeginPlay
  (|CallParentFunction))

(event EventTick
  (params (DeltaSeconds :type Float%20%28single-precision%29))
  (|CallParentFunction DeltaSeconds) ; This node is disabled and will not be called.\nDrag off pins to build functionality.
)

(event Collision|EventActorBeginOverlap
  (params (OtherActor :type Actor%20Object%20Reference)))

(fn ConstructionScript
  (|CallParentFunction)
  ;[1 1 1] Create blades and set new damage settings
  (Utilities|IsValid (Variables|Default|GetBP_ChildActor)
    (:Is%20Valid
      (bind _asbp_blades (Utilities|Casting|CastToBP_Blades (Variables|/Script/Engine.ChildActorComponent|GetChildActor (Variables|Default|GetBP_ChildActor))))
      (Variables|/Game/DeathTrapsVol_1/Blueprints/Traps/Blade/BP_Blades.BP_Blades_C|SetNumberOfBlades _asbp_blades (Variables|Settings|Blades|GetNumberOfBlades))
      (Default|CreateBlades _asbp_blades)
      (Default|SetNewDamagetoBlades _asbp_blades (Variables|Default|GetDamage) (Variables|Default|GetImpulse) (Variables|Default|GetbCustomImpulse) (Variables|Default|GetDamageType)))))