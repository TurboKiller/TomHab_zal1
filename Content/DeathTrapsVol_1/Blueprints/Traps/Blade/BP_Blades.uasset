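; BP_Blades is a trap part that builds a radial set of blade weapons for a death trap.
; CreateBlades adds child actor components of BladeClass at a set height, spaced evenly in yaw over 360 degrees, and stores them in BladesRef.
; SetNewDamageToBlades passes damage, impulse and damage type to each blade's BP_BaseModuleWeapon, printing an error on a failed cast.
; Its own events and construction script are empty.
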(event EventBeginPlay)

(event Collision|EventActorBeginOverlap
  (params (OtherActor :type Actor%20Object%20Reference)))

(event EventTick
  (params (DeltaSeconds :type Float%20%28single-precision%29)))

(fn ConstructionScript)

(fn SetNewDamagetoBlades
  (params (NewDamageBlades :type Float%20%28single-precision%29) (Impulse :type Vector) (bCustomImpulse :type Boolean) (DamageType :type Damage%20Type%20Class%20Reference))
  ;[1 1 1] Set each blade new damage
  (for _array_element (Variables|Settings|GetBladesRef)
    (bind _asbp_base_module_weapon (Utilities|Casting|CastToBP_BaseModuleWeapon (Variables|/Script/Engine.ChildActorComponent|GetChildActor _array_element))
      (:then
        (Default|SetNewDamage _asbp_base_module_weapon NewDamageBlades Impulse bCustomImpulse DamageType))
      (:CastFailed
        (Development|PrintString "*** BP_Blades: Fail cast to BP_BaseModularWeapon ***" true true "(R=0.000000,G=0.660000,B=1.000000,A=1.000000)" 1e+01)))))

(fn CreateBlades
  (bind _numberofblades (Variables|Blades|GetNumberOfBlades))
  ;[1 1 1] Create blades
  (Utilities|Array|Clear (Variables|Settings|GetBladesRef)) ; Clear blades ref
  (for _index (range 0 (- _numberofblades 1))
    (bind _returnvalue (AddComponent|AddChildActorComponent false (Math|Transform|MakeTransform (Math|Vector|MakeVector 0.0 0.0 (Variables|Blades|GetHeightBlades)) (Math|Rotator|MakeRotator 0.0 0.0 (* _index (/ 3.6e+02 (Math|Conversions|ToFloat(Integer) _numberofblades)))) "1,1,1")))
    (Utilities|Array|Add (Variables|Settings|GetBladesRef) _returnvalue)
    (ChildActorComponent|SetChildActorClass _returnvalue (Variables|Blades|GetBladeClass)) ; Set blade class
  ))