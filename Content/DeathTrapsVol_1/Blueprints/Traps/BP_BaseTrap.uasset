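; Base trap actor that plays a vector-curve-driven animation, with child actors supplying the motion by overriding AnimationLogic.
; Tick advances curve time forward, backward or ping-pong, counting each end as a repeat and optionally pausing between repeats via timer.
; It runs endlessly or for a set count after an optional random start delay.
; An optional linked trigger starts it, then is re-enabled when repeats finish, or destroyed for endless traps.
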(event Custom|OnActivateTrapAfterDelay
  ;[1 1 1] Activete tick by timer
  (bind _output_get (Variables|Settings|Animation|SetbActiveTrap true))
  (Actor|Tick|SetActorTickEnabled _output_get))

(event Custom|Trigger_Disp
  ;[1 1 1] If set trigger the trap will be disabled and has been activated by trigger
  (if (not (Variables|Settings|Animation|GetbActiveTrap))
    (CallFunction|ClalulateRandomDelay)
    (Utilities|FlowControl|Delay (Variables|Settings|DelayStart|GetDelayStart))
    (bind _output_get (Variables|Settings|Animation|SetbActiveTrap true))
    (Actor|Tick|SetActorTickEnabled _output_get)
    (Default|ActivateTrigger (Variables|Settings|GetTriggerRef) false) ; Deactivate trigger
    ;[1 0.8425 0] destroy the trigger if the trap is turned on for endless repetitions
    (if (Variables|Settings|Animation|GetbInfinityActivate)
      (Actor|DestroyActor (Variables|Settings|GetTriggerRef)))))

(event Custom|OnStartDelayTrap
  ;[1 1 1] Diasble tick and start delay timer
  (bind _output_get (Variables|Settings|Animation|SetbActiveTrap false))
  (Actor|Tick|SetActorTickEnabled _output_get)
  (bind _returnvalue (Utilities|Time|SetTimerbyEvent (EventDispatchers|CreateEvent :!event Custom|OnActivateTrapAfterDelay) (Variables|Settings|Animation|GetDelayBetweenRepeat)))
  (Variables|Settings|SetActivateTrapAfterDelay_TimerHandle _returnvalue))

(event EventBeginPlay
  (Utilities|FlowControl|Sequence
    (:then_0
      ;[1 1 1] Initialize started variable for animation from curve
      (Utilities|IsValid (Variables|Settings|Animation|GetCurveVectorAnimation)
        (:Is%20Valid
          (Variables|Settings|Animation|SetDurationAnimation (.MaxTime (Math|Curves|GetTimeRange (Variables|Settings|Animation|GetCurveVectorAnimation))))
          (Variables|Settings|Animation|SetTimeAnimation (Utilities|Select :Index (Variables|Settings|Animation|GetDirectionAnimation) :NewEnumerator0 0.0 :NewEnumerator1 0.0 :NewEnumerator2 (Variables|Settings|Animation|GetDurationAnimation)))
          (Variables|Settings|Animation|SetbForwardAnimation (Utilities|Select :Index (Variables|Settings|Animation|GetDirectionAnimation) :NewEnumerator0 true :NewEnumerator1 true :NewEnumerator2 false))
          (CallFunction|ClalulateRandomDelay)
          (Utilities|FlowControl|Delay (Variables|Settings|DelayStart|GetDelayStart))
          (Actor|Tick|SetActorTickEnabled (Variables|Settings|Animation|GetbActiveTrap)))))
    (:then_1
      ;[1 1 1] If set trigger the trap will be disabled and has been activated by trigger
      (Utilities|IsValid (Variables|Settings|GetTriggerRef)
        (:Is%20Valid
          (EventDispatchers|AssignTriggerDisp (Variables|Settings|GetTriggerRef) (delegate Custom|Trigger_Disp))
          (bind _output_get (Variables|Settings|Animation|SetbActiveTrap false))
          (Actor|Tick|SetActorTickEnabled _output_get))))))

(event EventTick
  (params (DeltaSeconds :type Float%20%28single-precision%29))
  (bind _triggerref (Variables|Settings|GetTriggerRef))
  ;[1 1 1] Caclulate animation each tick
  (DeathTraps|CalculateFrameAnimation)
  ;[1 1 1] Active trap all time
  (if (Variables|Settings|Animation|GetbInfinityActivate)
    (DeathTraps|AnimationLogic) ; Override this function on child actor
    (elif (DeathTraps|Continue)
      (DeathTraps|AnimationLogic) ; Override this function on child actor
      (else
        ;[1 1 1] Deactivate animation and reset CurrentRepeatAnimation
        (Variables|Settings|Animation|SetCurrentRepeatAnimation 0)
        (bind _output_get (Variables|Settings|Animation|SetbActiveTrap false))
        (Actor|Tick|SetActorTickEnabled _output_get)
        ;[1 1 1] Last tick
        (DeathTraps|AnimationLogic) ; Override this function on child actor
        ;[1 1 1] Activate trigger
        (Utilities|IsValid _triggerref
          (:Is%20Valid
            (Default|ActivateTrigger _triggerref true) ; Deactivate trigger
          )
          (:Is%20Not%20Valid
            _))
        ;[1 1 1] Deactivate the timer if all repeatings are done
        (if (not (Variables|Settings|Animation|GetbInfinityActivate)) ; Clear timer if InfinityActivate set False
          (Utilities|Time|ClearandInvalidateTimerbyHandle (Variables|Settings|GetActivateTrapAfterDelay_TimerHandle)))))))

(fn ConstructionScript
  (Utilities|FlowControl|Sequence
    (:then_0
      ;[1 1 1] If InfinityActivate set True then ActiveTrap set True
      (if (Variables|Settings|Animation|GetbInfinityActivate)
        (bind _output_get (Variables|Settings|Animation|SetbActiveTrap true))
        (Actor|Tick|SetActorTickEnabled _output_get)))
    (:then_1
      ;[1 1 1] If trigger is set then the trap deactivate by default
      (Utilities|IsValid (Variables|Settings|GetTriggerRef)
        (:Is%20Valid
          (bind _output_get_2 (Variables|Settings|Animation|SetbActiveTrap false))
          (Actor|Tick|SetActorTickEnabled _output_get_2))))))

(fn CalculateFrameAnimation
  ;[1 1 1] Calculate direction animation
  (bind _output_get (Variables|Settings|Animation|SetTimeAnimation (+ (Variables|Settings|Animation|GetTimeAnimation) (* (Utilities|Time|GetWorldDeltaSeconds) (select (Variables|Settings|Animation|GetbForwardAnimation) 1.0 -1.0)))))
  ;[1 1 1] Get frame animation (alpha)
  (Variables|Settings|Animation|SetFrameAnimation (Math|Curves|GetVectorValue (Variables|Settings|Animation|GetCurveVectorAnimation) _output_get))
  (switch Utilities|FlowControl|Switch|SwitchonE_DirectionsAnimation (Variables|Settings|Animation|GetDirectionAnimation)
    (:NewEnumerator0
      (bind _directionswitched (DeathTraps|ForwardBackwardDirectionLogic))
      (LocalVariables|SetbL_DirectionSwitched _directionswitched))
    (:NewEnumerator1
      (bind _directionswitched_2 (DeathTraps|ForwardDirectionLogic))
      (LocalVariables|SetbL_DirectionSwitched _directionswitched_2) ; to count the number of repetitions
    )
    (:NewEnumerator2
      (bind _directionswitched_3 (DeathTraps|BackwardDirectionLogic))
      (LocalVariables|SetbL_DirectionSwitched _directionswitched_3) ; to count the number of repetitions
    ))
  ;[1 1 1] If derection switched
  (if (LocalVariables|GetbL_DirectionSwitched)
    ;[1 1 1] Increase repeat animation
    (Variables|Settings|Animation|SetCurrentRepeatAnimation (+ (Variables|Settings|Animation|GetCurrentRepeatAnimation) 1))
    ;[1 1 1] If DelayBetweenAnimation > 0 then start delay before next animation
    (if (> (Variables|Settings|Animation|GetDelayBetweenRepeat) 0.0)
      (CallFunction|OnStartDelayTrap))))

(fn AnimationLogic)

(fn Continue
  (return (< (Variables|Settings|Animation|GetCurrentRepeatAnimation) (Variables|Settings|Animation|GetNumberRepeatAnimation))))

(fn ForwardBackwardDirectionLogic
  ;[1 1 1] Switch diection animation to backward
  (if (> (Variables|Settings|Animation|GetTimeAnimation) (Variables|Settings|Animation|GetDurationAnimation))
    (Variables|Settings|Animation|SetbForwardAnimation false)
    (Variables|Settings|Animation|SetTimeAnimation (Variables|Settings|Animation|GetDurationAnimation))
    (LocalVariables|SetbL_DirectionSwitched true)
    (else
      ;[1 1 1] Switch direction animation to forward
      (if (< (Variables|Settings|Animation|GetTimeAnimation) 0.0)
        (Variables|Settings|Animation|SetbForwardAnimation true)
        (Variables|Settings|Animation|SetTimeAnimation 0.0)
        (LocalVariables|SetbL_DirectionSwitched true))))
  (return (LocalVariables|GetbL_DirectionSwitched)))

(fn ForwardDirectionLogic
  ;[1 1 1] Switch diection animation to backward
  (if (> (Variables|Settings|Animation|GetTimeAnimation) (Variables|Settings|Animation|GetDurationAnimation))
    (Variables|Settings|Animation|SetTimeAnimation 0.0)
    (return true) ; Just begin from start
    (else
      (return false) ; Continue
    )))

(fn BackwardDirectionLogic
  ;[1 1 1] Switch direction animation to forward
  (if (< (Variables|Settings|Animation|GetTimeAnimation) 0.0)
    (Variables|Settings|Animation|SetTimeAnimation (Variables|Settings|Animation|GetDurationAnimation))
    (Variables|Settings|Animation|SetbForwardAnimation false)
    (return true) ; Just begin from start
    (else
      (return false) ; Continue
    )))

(fn ClalulateRandomDelay
  (if (Variables|Settings|DelayStart|GetbRandomDelayStart) ; If True then generate random delay
    (Variables|Settings|DelayStart|SetDelayStart (Math|Random|RandomFloatinRange (Variables|Settings|DelayStart|GetMinRandomDelayStart) (Variables|Settings|DelayStart|GetMaxRandomDelayStart))))
  (return))