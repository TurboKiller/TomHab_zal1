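; BP_SpikeLogRotation is a rotating spiked log trap that hurts the player on contact.
; It extends a parent Blueprint, passing BeginPlay and Tick through to it.
; The construction script sets the child actor's class from WeaponClass and picks its initial rotation from the animation direction.
; Box overlap with BP_ThirdPersonCharacter applies a small fixed amount of damage through the character's own damage function.
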(event OnComponentBeginOverlap(Box)
  (params (OverlappedComponent :type Primitive%20Component%20Object%20Reference) (OtherActor :type Actor%20Object%20Reference) (OtherComp :type Primitive%20Component%20Object%20Reference) (OtherBodyIndex :type Integer) (bFromSweep :type Boolean) (SweepResult :type Hit%20Result%20Structure%20%28by%20ref%29))
  (bind _asbp_third_person_character (Utilities|Casting|CastToBP_ThirdPersonCharacter OtherActor))
  (Default|MainCharacterRecieveDamage _asbp_third_person_character 5.0 "NewEnumerator0" "0, 0, 0"))

(event EventBeginPlay
  (|CallParentFunction))

(event EventTick
  (params (DeltaSeconds :type Float%20%28single-precision%29))
  (|CallParentFunction DeltaSeconds))

(fn ConstructionScript
  (bind _rotationstart (Variables|Default|GetRotationStart))
  (|CallParentFunction)
  (ChildActorComponent|SetChildActorClass (Variables|Default|GetBP_ChildActor) (Variables|Default|GetWeaponClass)) ; Set weapon class
  ;[1 1 1] Start rotation trap by direction animation
  (Transformation|SetRelativeRotation (Variables|Default|GetBP_ChildActor) (Utilities|Select :Index (Variables|Default|GetDirectionAnimation) :NewEnumerator0 _rotationstart :NewEnumerator1 _rotationstart :NewEnumerator2 (Variables|Default|GetRotationEnd)) false false))