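; Base trigger actor from the DeathTraps pack that signals when an actor overlaps it.
; The construction script adds a box, sphere or capsule collision component, chosen by a shape setting and placed with a configurable transform.
; An overlap fires the trigger dispatcher only while the active flag is set, with no filter on the overlapping actor.
; ActivateTrigger sets that flag to switch the trigger on or off.
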(event EventBeginPlay)

(event Collision|EventActorBeginOverlap
  (params (OtherActor :type Actor%20Object%20Reference))
  (if (Variables|Settings|GetbActiveTrigger)
    (Default|CallTriggerDisp)))

(event EventTick
  (params (DeltaSeconds :type Float%20%28single-precision%29)))

(fn ConstructionScript
  (switch Utilities|FlowControl|Switch|SwitchonE_ShapesCollision (Variables|Settings|GetUseShapeCollidsion)
    (:NewEnumerator0
      (AddComponent|AddBoxComponent false (Variables|Settings|GetTransformShapeCollision)))
    (:NewEnumerator1
      (AddComponent|AddSphereComponent false (Variables|Settings|GetTransformShapeCollision)))
    (:NewEnumerator2
      (AddComponent|AddCapsuleComponent false (Variables|Settings|GetTransformShapeCollision)))))

(fn ActivateTrigger
  (params (ActiveTrigger :type Boolean))
  (Variables|Settings|SetbActiveTrigger ActiveTrigger))